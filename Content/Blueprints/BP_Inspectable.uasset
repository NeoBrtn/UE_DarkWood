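; Interactable actor that toggles between being held in front of the player's camera for inspection and being released.
; Interact disables the Cube's physics and attaches to the camera manager at a fixed forward offset, aligned to its rotation.
; Interacting again detaches, re-enables physics and applies the stored transform, which is the camera's at pickup rather than the object's.
; A short delay gates repeated interaction, and the interact prompt is empty.
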(event `/Game/Blueprints/Interfaces/BPI_Interactable.Interact`
  (params (Caller :type "Actor Object Reference"))
  (bind _playercameramanager (`PlayerController.PlayerCameraManager` (`GameplayStatics.GetPlayerController` 0)))
  (if (`self.CanInteract`)
    (set `self.CanInteract` false)
    (if (`self.Inspecting`)
      (set `self.Inspecting` false)
      (`self.K2_DetachFromActor` "KeepRelative")
      (`PrimitiveComponent.SetSimulatePhysics` (`self.Cube`) true)
      (`self.K2_SetActorTransform` (`self.OriginalTransform`))
      (`KismetSystemLibrary.Delay` 0.4)
      (set `self.CanInteract` true)
      (else
        (set `self.Inspecting` true)
        (set `self.OriginalTransform` (`self.GetTransform` _playercameramanager))
        (`PrimitiveComponent.SetSimulatePhysics` (`self.Cube`) false)
        (`self.K2_SetActorLocation` (+ (`PlayerCameraManager.GetCameraLocation` _playercameramanager) (* (`self.GetActorForwardVector` _playercameramanager) (`self.Distance`))))
        (`self.K2_SetActorRotation` (`self.K2_GetActorRotation` _playercameramanager))
        (`self.K2_AttachToComponent` (`Actor.RootComponent` _playercameramanager) "None" "KeepRelative" "KeepRelative" "KeepRelative")
        (`self.K2_SetActorRelativeLocation` (150.0 0.0 0.0))
        (`KismetSystemLibrary.Delay` 0.4)
        (set `self.CanInteract` true)))))

(fn `GetInteractPrompt`
  (returns (Prompt :type Text))
  (return ""))

(fn `UserConstructionScript`)