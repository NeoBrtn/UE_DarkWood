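; BP_HorrorCharacter is a first-person player character for a horror game, with movement, mouse look, a toggleable flashlight and interaction.
; Enhanced Input drives these actions through the IMC_Darkwood mapping context added on BeginPlay, with mouse look scaled by LookSensitivity.
; Every Tick, a short Visibility line trace from the camera along control rotation stores the hit actor as CurrentInteractable.
; The interact input sends that actor an interface message when it is valid.
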(event `EnhancedInput|/Game/Input/Actions/IA_Move`
  (params (ActionValue :type "Vector2D Structure") (ElapsedSeconds :type "Float (double-precision)") (TriggeredSeconds :type "Float (double-precision)") (InputAction :type "InputAction Object Reference" :default "/Game/Input/Actions/IA_Move.IA_Move"))
  (:`Triggered`
    (`self.AddMovementInput` (`self.GetActorForwardVector`) ActionValue_Y)
    (`self.AddMovementInput` (`self.GetActorRightVector`) ActionValue_X)))

(event `EnhancedInput|/Game/Input/Actions/IA_MouseLook`
  (params (ActionValue :type "Vector2D Structure") (ElapsedSeconds :type "Float (double-precision)") (TriggeredSeconds :type "Float (double-precision)") (InputAction :type "InputAction Object Reference" :default "/Game/Input/Actions/IA_MouseLook.IA_MouseLook"))
  (bind _looksensitivity (`self.LookSensitivity`))
  (:`Triggered`
    (`self.AddControllerYawInput` (* _looksensitivity ActionValue_X))
    (`self.AddControllerPitchInput` (* ActionValue_Y (* _looksensitivity -1.0)))))

(event `EnhancedInput|/Game/Input/Actions/IA_Interact`
  (params (ActionValue :type Boolean) (ElapsedSeconds :type "Float (double-precision)") (TriggeredSeconds :type "Float (double-precision)") (InputAction :type "InputAction Object Reference" :default "/Game/Input/Actions/IA_Interact.IA_Interact"))
  (bind _currentinteractable (`self.CurrentInteractable`))
  (:`Triggered`
    (`/Engine/EditorBlueprintResources/StandardMacros.IsValid` _currentinteractable
      (:`Is Valid`
        (message `/Game/Blueprints/Interfaces/BPI_Interactable.Interact` _currentinteractable self)))))

(event `self.ReceiveBeginPlay`
  (`EnhancedInputSubsystemInterface.AddMappingContext` (pcsubsystem `EnhancedInputLocalPlayerSubsystem` (`GameplayStatics.GetPlayerController` 0)) "/Game/Input/IMC_Darkwood.IMC_Darkwood" 0 (struct)))

(event `EnhancedInput|/Game/Input/Actions/IA_FlashLight`
  (params (ActionValue :type Boolean) (ElapsedSeconds :type "Float (double-precision)") (TriggeredSeconds :type "Float (double-precision)") (InputAction :type "InputAction Object Reference" :default "/Game/Input/Actions/IA_FlashLight.IA_FlashLight"))
  (:`Started`
    (`SceneComponent.ToggleVisibility` (`self.flashlight`) false)))

(event `self.ReceiveTick`
  (params (DeltaSeconds :type "Float (single-precision)"))
  (bind _returnvalue (`SceneComponent.K2_GetComponentLocation` (`self.Camera`)))
  (bind _outhit (`KismetSystemLibrary.LineTraceSingle` _returnvalue (+ _returnvalue (* (`KismetMathLibrary.GetForwardVector` (`self.GetControlRotation`)) 250.0)) "TraceTypeQuery1" false (`|MakeArray` null :!type "Actor Object Reference")))
  (set `self.CurrentInteractable` (`.HitActor` (`GameplayStatics.BreakHitResult` _outhit))))

(fn `UserConstructionScript`)